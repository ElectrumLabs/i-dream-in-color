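; BP_StairsPortal is an interactable stairs portal that moves the player character, Grigory, to a linked destination actor.
; On interaction it stores Grigory and opens a door click menu widget at the screen projection of its cube, unless one already exists.
; The menu receives the portal as its interactable reference, and the SelectedAction event teleports Grigory to the StairsDestination location without sweeping.
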(event Custom|CreateClickMenu
  ;[1 1 1] Create UI for player to select next course of action
  (Utilities|IsValid (Variables|Default|GetClickMenuREF)
    (:Is%20Valid
      (if (not (Variables|/Game/IDreamInColor/UI/ClickMenu/WBP_ClickMenu_Door.WBP_ClickMenu_Door_C|GetbExists (Variables|Default|GetClickMenuREF)))
        (bind _returnvalue (UserInterface|CreateWidget "/Game/IDreamInColor/UI/ClickMenu/WBP_ClickMenu_Door.WBP_ClickMenu_Door_C" 0 (.ScreenPosition (Class|GameplayStatics|ProjectWorldtoScreen (Game|GetPlayerController 0) (Transformation|GetWorldLocation (Variables|Default|GetCube)) false)) self :!label _label))
        (Variables|Default|SetClickMenuREF _returnvalue)
        (UserInterface|Viewport|AddtoViewport (Variables|Default|GetClickMenuREF) 0)))
    (:Is%20Not%20Valid
      (goto _label))))

(event EventSelectedAction
  (Transformation|SetActorLocation (Variables|Default|GetGrigoryREF) (Transformation|GetActorLocation (Variables|Default|GetStairsDestination)) false false))

(event EventPlayerInteraction
  (params (Grigory :type Grigory%20Object%20Reference))
  (Variables|Default|SetGrigoryREF Grigory)
  (CallFunction|CreateClickMenu))

(fn ConstructionScript)