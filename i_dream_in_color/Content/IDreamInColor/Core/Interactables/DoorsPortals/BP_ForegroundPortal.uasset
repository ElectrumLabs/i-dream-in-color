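; Foreground portal interactable that opens a door click menu when the player interacts, then slides the player character Grigory toward a destination.
; The menu widget spawns at the Cube's projected screen position, with a check against an existing menu.
; SelectedAction starts a looping timer that nudges Grigory along +X until reaching DoorDestination's X, printing a debug string each step.
; The timer is never cleared, and movement ignores Y, Z and collision sweeps.
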(event Custom|CreateClickMenu
  ;[1 1 1] Create UI for player to select next course of action
  (Utilities|IsValid (Variables|Default|GetClickMenuREF)
    (:Is%20Valid
      (if (not (Variables|/Game/IDreamInColor/UI/ClickMenu/WBP_ClickMenu_Door.WBP_ClickMenu_Door_C|GetbExists (Variables|Default|GetClickMenuREF)))
        (bind _returnvalue (UserInterface|CreateWidget "/Game/IDreamInColor/UI/ClickMenu/WBP_ClickMenu_Door.WBP_ClickMenu_Door_C" 0 (.ScreenPosition (Class|GameplayStatics|ProjectWorldtoScreen (Game|GetPlayerController 0) (Transformation|GetWorldLocation (Variables|Default|GetCube)) false)) self :!label _label))
        (Variables|Default|SetClickMenuREF _returnvalue)
        (UserInterface|Viewport|AddtoViewport (Variables|Default|GetClickMenuREF) 0)))
    (:Is%20Not%20Valid
      (goto _label))))

(event Custom|MovingAnimationProxy
  (bind _grigoryref (Variables|Default|GetGrigoryREF))
  (bind _returnvalue (Transformation|GetActorLocation _grigoryref))
  (if (< (.x _returnvalue) (.x (Transformation|GetActorLocation (Variables|Default|GetDoorDestination))))
    (Transformation|SetActorLocation (Variables|Default|GetGrigoryREF) (Math|Vector|MakeVector (+ (.x _returnvalue) 5.0) (.y _returnvalue) (.z _returnvalue)) false false)
    (Development|PrintString "Hello")))

(event EventSelectedAction
  (Utilities|Time|SetTimerbyEvent (delegate Custom|MovingAnimationProxy) 0.01 true))

(event EventPlayerInteraction
  (params (Grigory :type Grigory%20Object%20Reference))
  (Variables|Default|SetGrigoryREF Grigory)
  (CallFunction|CreateClickMenu))

(fn ConstructionScript)