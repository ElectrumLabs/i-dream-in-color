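; Interactable door that moves Grigory between two linked points and switches the axis plane he moves along.
; Player interaction stores Grigory and opens a click menu widget at the door's projected screen position, unless one already exists.
; The selected action checks his plane state, teleports him to the destination or starting point raised by capsule half-height, shifts his movement axis and updates the Traverse flag.
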(event Custom|CreateClickMenu
  ;[1 1 1] Create UI for player to select next course of action
  (Utilities|IsValid (Variables|Default|GetClickMenuREF)
    (:Is%20Valid
      (if (not (Variables|/Game/IDreamInColor/UI/ClickMenu/WBP_ClickMenu_Door.WBP_ClickMenu_Door_C|GetbExists (Variables|Default|GetClickMenuREF)))
        (bind _returnvalue (UserInterface|CreateWidget "/Game/IDreamInColor/UI/ClickMenu/WBP_ClickMenu_Door.WBP_ClickMenu_Door_C" 0 (.ScreenPosition (Class|GameplayStatics|ProjectWorldtoScreen (Game|GetPlayerController 0) (Transformation|GetWorldLocation (Variables|Default|GetStaticMesh)) false)) self :!label _label))
        (Variables|Default|SetClickMenuREF _returnvalue)
        (UserInterface|Viewport|AddtoViewport (Variables|Default|GetClickMenuREF) 0)))
    (:Is%20Not%20Valid
      (goto _label))))

(event EventPlayerInteraction
  (params (Grigory :type Grigory%20Object%20Reference))
  (CallFunction|CreateClickMenu)
  (Variables|Default|SetGrigoryREF Grigory))

(event EventSelectedAction
  (bind _doordestination (Variables|Default|GetDoorDestination))
  (bind _grigoryref (Variables|Default|GetGrigoryREF))
  (bind _doorstartingpoint (Variables|Default|GetDoorStartingPoint))
  (bind _returnvalue (Transformation|GetActorLocation _doordestination))
  (bind _returnvalue_2 (Transformation|GetActorLocation _doorstartingpoint))
  (switch Utilities|FlowControl|Switch|SwitchonEPlaneState (Variables|/Game/IDreamInColor/Core/Characters/Grigory.Grigory_C|GetPlaneState _grigoryref)
    (:NewEnumerator0
      (Transformation|SetActorLocation _grigoryref (Math|Vector|MakeVector (.x _returnvalue) (.y _returnvalue) (+ (.z _returnvalue) (Components|Capsule|GetScaledCapsuleHalfHeight (Variables|/Script/Engine.Character|GetCapsuleComponent _grigoryref)))) false false)
      (Default|ShiftX _grigoryref)
      (Variables|Default|SetbTraverse false))
    (:NewEnumerator1
      (Transformation|SetActorLocation _grigoryref (Math|Vector|MakeVector (.x _returnvalue_2) (.y _returnvalue_2) (+ (.z _returnvalue_2) (Components|Capsule|GetScaledCapsuleHalfHeight (Variables|/Script/Engine.Character|GetCapsuleComponent _grigoryref)))) false false)
      (Default|ShiftY _grigoryref)
      (Variables|Default|SetbTraverse true))))

(fn ConstructionScript
  (|CallParentFunction))