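; BP_CueTrigger is an overlap trigger that plays a dialogue cue when the Grigory character enters it.
; It plays the dialogue at Grigory's location using a speaker and audience context.
; If a quest row is set, it looks up that objectives table row and adds it uniquely to the game instance's objectives.
; It can optionally destroy itself after triggering so the cue plays only once.
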(event Custom|AddObjective
  (bind _returnvalue (Utilities|GetDataTableRow "/Game/IDreamInColor/Core/Questlines/ObjectivesTable.ObjectivesTable" (Variables|Default|GetQuestRowIndex))
    (:then
      (Utilities|Array|AddUnique (Variables|/Game/IDreamInColor/Core/IDICGameInstance.IDICGameInstance_C|GetObjectives (Variables|Default|GetGameInstanceREF)) _returnvalue))))

(event EventBeginPlay
  ;[1 1 1] Constructor
  (bind _asidicgame_instance (Utilities|Casting|CastToIDICGameInstance (Game|GetGameInstance)))
  (Variables|Default|SetGameInstanceREF _asidicgame_instance))

(event Collision|EventActorBeginOverlap
  (params (OtherActor :type Actor%20Object%20Reference))
  ;[1 1 1] Play dialogue
  (bind _asgrigory (Utilities|Casting|CastToGrigory OtherActor))
  (Variables|Default|SetbIsTriggered true)
  (Class|GameplayStatics|PlayDialogueatLocation (Variables|Default|GetDialogue) (Utilities|Struct|MakeDialogueContext (Variables|Default|GetSpeaker) (Variables|Default|GetAudience)) (Transformation|GetActorLocation _asgrigory) "0, 0, 0" 1.0 1.0 0.0 0)
  ;[1 0.8541 0.2474] Comment
  (if (Utilities|Name|NotEqual(Name) (Variables|Default|GetQuestRowIndex) "None")
    (CallFunction|AddObjective))
  ;[1 1 1] Self destruct
  (if (Variables|Default|GetbPlayOnce)
    (Actor|DestroyActor)))

(fn ConstructionScript)