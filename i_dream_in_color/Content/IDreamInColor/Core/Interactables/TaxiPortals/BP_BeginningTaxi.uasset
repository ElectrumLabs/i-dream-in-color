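; BP_BeginningTaxi is an interactable taxi that opens a travel menu for the player.
; Interaction spawns a door-style click menu at the taxi mesh's projected screen position, skipping creation if one already exists.
; The selected action creates the beginning travel menu with a reference to the taxi and switches input to Game and UI.
; Close clears the InBound flag and removes the travel menu.
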(event Custom|CreateClickMenu
  ;[1 1 1] Create UI for player to select next course of action
  (Utilities|IsValid (Variables|Default|GetClickMenuREF)
    (:Is%20Valid
      (if (not (Variables|/Game/IDreamInColor/UI/ClickMenu/WBP_ClickMenu_Door.WBP_ClickMenu_Door_C|GetbExists (Variables|Default|GetClickMenuREF)))
        (bind _returnvalue (UserInterface|CreateWidget "/Game/IDreamInColor/UI/ClickMenu/WBP_ClickMenu_Door.WBP_ClickMenu_Door_C" 0 (.ScreenPosition (Class|GameplayStatics|ProjectWorldtoScreen (Game|GetPlayerController 0) (Transformation|GetWorldLocation (Variables|Default|GetTaxiMesh)) false)) self :!label _label))
        (Variables|Default|SetClickMenuREF _returnvalue)
        (UserInterface|Viewport|AddtoViewport (Variables|Default|GetClickMenuREF) 0)))
    (:Is%20Not%20Valid
      (goto _label))))

(event Custom|Close
  (Variables|Default|SetinBound false)
  (Utilities|IsValid (Variables|Default|GetTravelWidgetREF)
    (:Is%20Valid
      (Widget|RemovefromParent (Variables|Default|GetTravelWidgetREF))
      (Variables|Default|SetTravelWidgetREF 0))))

(event EventPlayerInteraction
  (params (Grigory :type Grigory%20Object%20Reference))
  (CallFunction|CreateClickMenu))

(event EventSelectedAction
  (bind _returnvalue (UserInterface|CreateWidget "/Game/IDreamInColor/UI/BegnningTravelMenuWidget.BegnningTravelMenuWidget_C" (Game|GetPlayerController 0) self))
  (bind _output_get (Variables|Default|SetTravelWidgetREF _returnvalue))
  (UserInterface|Viewport|AddtoViewport _output_get 0)
  (Input|SetInputModeGameandUI (Game|GetPlayerController 0) 0 "DoNotLock" true))

(fn ConstructionScript)