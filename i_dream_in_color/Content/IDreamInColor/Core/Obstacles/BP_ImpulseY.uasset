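; BP_ImpulseY is an obstacle that shuttles its Cube along world Y, out by Range from its start position and back.
; BeginPlay records the start Y and starts a looping 0.01-second timer, using mirrored step events chosen by the sign of Speed.
; Back at the start, the movement timer pauses until a one-shot PauseTimer delay resumes it.
; The Box overlap only casts to SideScrollerCharacter and does nothing further.
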(event OnComponentBeginOverlap(Box)
  (params (OverlappedComponent :type Primitive%20Component%20Object%20Reference) (OtherActor :type Actor%20Object%20Reference) (OtherComp :type Primitive%20Component%20Object%20Reference) (OtherBodyIndex :type Integer) (bFromSweep :type Boolean) (SweepResult :type Hit%20Result%20Structure%20%28by%20ref%29))
  (Utilities|Casting|CastToSideScrollerCharacter OtherActor))

(event Custom|ReverseGoingUp
  (bind _cube (Variables|Default|GetCube))
  (bind _cube_2 (Variables|Default|GetCube))
  (bind _returnvalue (Transformation|GetWorldLocation _cube_2))
  (bind _returnvalue_2 (Transformation|GetWorldLocation _cube))
  (if (and (> (.y (Transformation|GetWorldLocation (Variables|Default|GetCube))) (- (Variables|Default|GetOriginalY) (Variables|Default|GetRange))) (Variables|Default|GetbGoingUp))
    (Transformation|SetWorldLocation _cube_2 (Math|Vector|MakeVector (.x _returnvalue) (+ (.y _returnvalue) (* 1.0 (Variables|Default|GetSpeed))) (.z _returnvalue)) false false)
    (else
      (Variables|Default|SetbGoingUp false)
      (if (<= (.y (Transformation|GetWorldLocation (Variables|Default|GetCube))) (Variables|Default|GetOriginalY))
        (Transformation|SetWorldLocation _cube (Math|Vector|MakeVector (.x _returnvalue_2) (- (.y _returnvalue_2) (* 1.0 (Variables|Default|GetSpeed))) (.z _returnvalue_2)) false false)
        (else
          (Utilities|Time|PauseTimerbyHandle (Variables|Default|GetElevatorTimer))
          (Utilities|Time|SetTimerbyEvent (delegate Custom|ReverseGoingDown) (Variables|Default|GetPauseTimer)))))))

(event Custom|Rise
  (bind _cube (Variables|Default|GetCube))
  (bind _cube_2 (Variables|Default|GetCube))
  (bind _returnvalue (Transformation|GetWorldLocation _cube))
  (bind _returnvalue_2 (Transformation|GetWorldLocation _cube_2))
  (if (and (<= (.y _returnvalue) (+ (Variables|Default|GetOriginalY) (Variables|Default|GetRange))) (Variables|Default|GetbGoingUp))
    (Transformation|SetWorldLocation _cube (Math|Vector|MakeVector (.x _returnvalue) (+ (.y _returnvalue) (* 1.0 (Variables|Default|GetSpeed))) (.z _returnvalue)) false false)
    (else
      (Variables|Default|SetbGoingUp false)
      (if (> (.y (Transformation|GetWorldLocation (Variables|Default|GetCube))) (Variables|Default|GetOriginalY))
        (Transformation|SetWorldLocation _cube_2 (Math|Vector|MakeVector (.x _returnvalue_2) (- (.y _returnvalue_2) (* 1.0 (Variables|Default|GetSpeed))) (.z _returnvalue_2)) false false)
        (else
          (Utilities|Time|PauseTimerbyHandle (Variables|Default|GetElevatorTimer))
          (Utilities|Time|SetTimerbyEvent (delegate Custom|UnpauseTimer) (Variables|Default|GetPauseTimer)))))))

(event Custom|UnpauseTimer
  ;[1 1 1] Unpause the pause
  (Variables|Default|SetbGoingUp true)
  (Utilities|Time|UnpauseTimerbyHandle (Variables|Default|GetElevatorTimer)))

(event Custom|ReverseGoingDown
  ;[1 1 1] Unpause the pause
  (Variables|Default|SetbGoingUp true)
  (Utilities|Time|UnpauseTimerbyHandle (Variables|Default|GetElevatorTimer)))

(event EventBeginPlay
  (Variables|Default|SetOriginalY (.y (Transformation|GetWorldLocation (Variables|Default|GetCube))))
  (if (< (Variables|Default|GetSpeed) 0.0)
    (bind _returnvalue (Utilities|Time|SetTimerbyEvent (delegate Custom|ReverseGoingUp) 0.01 true))
    (Variables|Default|SetElevatorTimer _returnvalue)
    (else
      (bind _returnvalue_2 (Utilities|Time|SetTimerbyEvent (delegate Custom|Rise) 0.01 true))
      (Variables|Default|SetElevatorTimer _returnvalue_2))))

(fn ConstructionScript)