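; BP_ReverseDisappearer is a minor obstacle whose cube toggles visibility while the SideScrollerCharacter overlaps the actor.
; Begin and end overlap each call SetStatus to flip the cube's visibility, so leaving undoes the change made on entering.
; The SetOff flag guards against repeated triggers, and the Visible flag tracks the current state.
; Only visibility changes; the graph leaves collision untouched.
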(event Custom|SetStatus
  (bind _cube (Variables|Default|GetCube))
  (if (Variables|Default|GetbVisible)
    (Rendering|SetVisibility _cube false false)
    (Variables|Default|SetbVisible false)
    (else
      (Rendering|SetVisibility _cube true false)
      (Variables|Default|SetbVisible true))))

(event Collision|EventActorEndOverlap
  (params (OtherActor :type Actor%20Object%20Reference))
  (Utilities|Casting|CastToSideScrollerCharacter OtherActor)
  (if (Variables|Default|GetbSetOff)
    (CallFunction|SetStatus)
    (Variables|Default|SetbSetOff false)))

(event Collision|EventActorBeginOverlap
  (params (OtherActor :type Actor%20Object%20Reference))
  (Utilities|Casting|CastToSideScrollerCharacter OtherActor)
  (if (not (Variables|Default|GetbSetOff))
    (CallFunction|SetStatus)
    (Variables|Default|SetbSetOff true)))

(fn ConstructionScript)