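; Obstacle platform that warns and then vanishes after the side-scroller character overlaps it, returning after a delay.
; Timer events swap the cube to a warning material, hide it and disable its collision, then restore its grey material, visibility and collision.
; While it is gone, a Box overlap pauses the reappear timer and blocks respawning until the overlap ends, so it does not return inside an occupant.
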(event OnComponentBeginOverlap(Box)
  (params (OverlappedComponent :type Primitive%20Component%20Object%20Reference) (OtherActor :type Actor%20Object%20Reference) (OtherComp :type Primitive%20Component%20Object%20Reference) (OtherBodyIndex :type Integer) (bFromSweep :type Boolean) (SweepResult :type Hit%20Result%20Structure%20%28by%20ref%29))
  (if (Variables|Default|GetbSetOff)
    (Utilities|Time|PauseTimerbyHandle (Variables|Default|GetReappearTimer))
    (Variables|Default|SetbCanSpawn false)))

(event OnComponentEndOverlap(Box)
  (params (OverlappedComponent :type Primitive%20Component%20Object%20Reference) (OtherActor :type Actor%20Object%20Reference) (OtherComp :type Primitive%20Component%20Object%20Reference) (OtherBodyIndex :type Integer))
  (Utilities|Time|UnpauseTimerbyHandle (Variables|Default|GetReappearTimer))
  (Variables|Default|SetbCanSpawn true))

(event Custom|Reappear
  (bind _cube (Variables|Default|GetCube))
  (if (Variables|Default|GetbCanSpawn)
    (Rendering|Material|SetMaterial (Variables|Default|GetCube) 0 "/Game/IDreamInColor/Character/SideScrollerCharacter/Painting/GreyMat.GreyMat")
    (Collision|SetCollisionEnabled _cube "QueryAndPhysics")
    (Rendering|SetVisibility _cube true false)
    (Variables|Default|SetbInvisible false)
    (Variables|Default|SetbSetOff false)))

(event Custom|Disappear
  (bind _cube (Variables|Default|GetCube))
  (Collision|SetCollisionEnabled _cube "NoCollision")
  (Rendering|SetVisibility _cube false false)
  (Variables|Default|SetbInvisible true)
  (Variables|Default|SetbSetOff true)
  (bind _returnvalue (Utilities|Time|SetTimerbyEvent (delegate Custom|Reappear) (Variables|Default|GetReappearTime)))
  (Variables|Default|SetReappearTimer _returnvalue))

(event Custom|SetStatus
  (if (not (Variables|Default|GetbInvisible))
    (Rendering|Material|SetMaterial (Variables|Default|GetCube) 0 "/Game/IDreamInColor/Core/Obstacles/Materials/M_Warning.M_Warning")
    (Utilities|Time|SetTimerbyEvent (delegate Custom|Disappear) (Variables|Default|GetWarningTime))))

(event Collision|EventActorBeginOverlap
  (params (OtherActor :type Actor%20Object%20Reference))
  (Utilities|Casting|CastToSideScrollerCharacter OtherActor)
  (if (not (Variables|Default|GetbSetOff))
    (Utilities|Time|SetTimerbyEvent (delegate Custom|SetStatus) 0.01)))

(fn ConstructionScript)