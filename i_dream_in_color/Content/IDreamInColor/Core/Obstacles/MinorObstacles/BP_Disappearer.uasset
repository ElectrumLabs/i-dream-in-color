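; BP_Disappearer is an obstacle whose cube periodically vanishes and reappears.
; A looping timer either switches the visible cube to a warning material and schedules its disappearance, or restores an invisible cube's grey material, collision and visibility.
; Disappearing hides the cube and disables its collision.
; A Box overlap with the SideScrollerCharacter blocks respawning, so an invisible cube waits for a later timer tick after the character leaves.
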(event OnComponentBeginOverlap(Box)
  (params (OverlappedComponent :type Primitive%20Component%20Object%20Reference) (OtherActor :type Actor%20Object%20Reference) (OtherComp :type Primitive%20Component%20Object%20Reference) (OtherBodyIndex :type Integer) (bFromSweep :type Boolean) (SweepResult :type Hit%20Result%20Structure%20%28by%20ref%29))
  (Utilities|Casting|CastToSideScrollerCharacter OtherActor)
  (Variables|Default|SetbCanSpawn false))

(event OnComponentEndOverlap(Box)
  (params (OverlappedComponent :type Primitive%20Component%20Object%20Reference) (OtherActor :type Actor%20Object%20Reference) (OtherComp :type Primitive%20Component%20Object%20Reference) (OtherBodyIndex :type Integer))
  (Utilities|Casting|CastToSideScrollerCharacter OtherActor)
  (Variables|Default|SetbCanSpawn true))

(event Custom|SetStatus
  (bind _cube (Variables|Default|GetCube))
  (if (Variables|Default|GetbInvisible)
    (if (Variables|Default|GetbCanSpawn)
      (Rendering|Material|SetMaterial (Variables|Default|GetCube) 0 "/Game/IDreamInColor/Character/SideScrollerCharacter/Painting/GreyMat.GreyMat")
      (Collision|SetCollisionEnabled _cube "QueryAndPhysics")
      (Rendering|SetVisibility _cube true false)
      (Variables|Default|SetbInvisible false))
    (else
      (Rendering|Material|SetMaterial (Variables|Default|GetCube) 0 "/Game/IDreamInColor/Core/Obstacles/Materials/M_Warning.M_Warning")
      (Utilities|Time|SetTimerbyEvent (delegate Custom|Disappear) (Variables|Default|GetWarningTime)))))

(event Custom|Disappear
  (bind _cube (Variables|Default|GetCube))
  (Collision|SetCollisionEnabled _cube "NoCollision")
  (Rendering|SetVisibility _cube false false)
  (Variables|Default|SetbInvisible true))

(event EventBeginPlay
  (Utilities|Time|SetTimerbyEvent (delegate Custom|SetStatus) (Variables|Default|GetPreWarningTime) true))

(fn ConstructionScript)