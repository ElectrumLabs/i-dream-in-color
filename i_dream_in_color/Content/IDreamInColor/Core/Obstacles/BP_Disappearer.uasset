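; BP_Disappearer is an obstacle cube that periodically vanishes and reappears.
; A looping timer set at BeginPlay calls SetStatus, which toggles on the Invisible flag.
; When visible, it switches to a warning material, waits a warning delay, then hides the cube and disables its collision.
; When invisible, it restores the grey material, collision and visibility.
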(event Custom|SetStatus
  (bind _cube (Variables|Default|GetCube))
  (bind _cube_2 (Variables|Default|GetCube))
  (if (Variables|Default|GetbInvisible)
    (Rendering|Material|SetMaterial (Variables|Default|GetCube) 0 "/Game/IDreamInColor/Character/SideScrollerCharacter/Painting/GreyMat.GreyMat")
    (Collision|SetCollisionEnabled _cube "QueryAndPhysics")
    (Rendering|SetVisibility _cube true false)
    (Variables|Default|SetbInvisible false)
    (else
      (Rendering|Material|SetMaterial (Variables|Default|GetCube) 0 "/Game/IDreamInColor/Core/Obstacles/Materials/M_Warning.M_Warning")
      (Utilities|FlowControl|Delay (Variables|Default|GetWarningTime))
      (Collision|SetCollisionEnabled _cube_2 "NoCollision")
      (Rendering|SetVisibility _cube_2 false false)
      (Variables|Default|SetbInvisible true))))

(event EventBeginPlay
  (Utilities|Time|SetTimerbyEvent (delegate Custom|SetStatus) (Variables|Default|GetPreWarningTime) true))

(fn ConstructionScript)