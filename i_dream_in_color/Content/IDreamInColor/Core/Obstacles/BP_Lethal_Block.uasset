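; Lethal obstacle block that kills the Grigory player character and respawns it at a checkpoint.
; Caches the IDIC game instance on BeginPlay.
; KillPlayer destroys the passed Grigory, has the game instance spawn a new one at ArcoriasCheckpoint, and prints a debug string.
; Nothing in this Blueprint calls KillPlayer, and it has no overlap or hit handling of its own.
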(event EventBeginPlay
  (bind _asidicgame_instance (Utilities|Casting|CastToIDICGameInstance (Game|GetGameInstance)))
  (Variables|Default|SetGameInstanceREF _asidicgame_instance))

(event EventKillPlayer
  (params (GrigoryREF :type Side%20Scroller%20Character%20Object%20Reference))
  (bind _gameinstanceref (Variables|Default|GetGameInstanceREF))
  (Actor|DestroyActor GrigoryREF)
  (Default|SpawnGrigory _gameinstanceref (Variables|/Game/IDreamInColor/Core/IDICGameInstance.IDICGameInstance_C|GetArcoriasCheckpoint _gameinstanceref))
  (Development|PrintString "Hello"))

(fn ConstructionScript
  (|CallParentFunction))