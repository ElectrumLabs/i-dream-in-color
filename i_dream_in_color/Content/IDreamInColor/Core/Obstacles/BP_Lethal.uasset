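; BP_Lethal is an obstacle that kills the side-scroller player character when it hits the obstacle.
; The Box component's hit event casts the other actor to SideScrollerCharacter and passes it to KillPlayer.
; KillPlayer destroys a valid character, then HandleDeathScreen creates WBP_DeathScreen, stores a reference and adds it to the viewport.
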(event OnComponentHit(Box)
  (params (HitComponent :type Primitive%20Component%20Object%20Reference) (OtherActor :type Actor%20Object%20Reference) (OtherComp :type Primitive%20Component%20Object%20Reference) (NormalImpulse :type Vector :default "0, 0, 0") (Hit :type Hit%20Result%20Structure%20%28by%20ref%29))
  (bind _asside_scroller_character (Utilities|Casting|CastToSideScrollerCharacter OtherActor))
  (CallFunction|KillPlayer _asside_scroller_character))

(event Custom|KillPlayer
  (params (GrigoryREF :type Side%20Scroller%20Character%20Object%20Reference))
  (Utilities|IsValid GrigoryREF
    (:Is%20Valid
      (Actor|DestroyActor GrigoryREF)
      (CallFunction|HandleDeathScreen))))

(event Custom|HandleDeathScreen
  (bind _returnvalue (UserInterface|CreateWidget "/Game/IDreamInColor/UI/WBP_DeathScreen.WBP_DeathScreen_C"))
  (Variables|Default|SetDeathScreenREF _returnvalue)
  (UserInterface|Viewport|AddtoViewport (Variables|Default|GetDeathScreenREF) 0))

(fn ConstructionScript)