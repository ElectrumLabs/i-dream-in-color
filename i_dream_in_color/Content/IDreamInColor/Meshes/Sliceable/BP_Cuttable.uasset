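; Cuttable actor that gets sliced in two by any component that begins overlapping its procedural mesh.
; On BeginPlay it copies the Mesh2Slice static mesh into a procedural mesh with collision.
; Each overlap slices that mesh on a plane set by the other component's location and forward vector, capping the cut with a new material section.
; Only the newly created half is set to simulate physics.
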(event OnComponentBeginOverlap(ProceduralMesh)
  (params (OverlappedComponent :type Primitive%20Component%20Object%20Reference) (OtherActor :type Actor%20Object%20Reference) (OtherComp :type Primitive%20Component%20Object%20Reference) (OtherBodyIndex :type Integer) (bFromSweep :type Boolean) (SweepResult :type Hit%20Result%20Structure%20%28by%20ref%29))
  ;[1 1 1] Slice
  (bind _outotherhalfprocmesh (Class|KismetProceduralMeshLibrary|SliceProceduralMesh (Variables|Default|GetProceduralMesh) (Transformation|GetWorldLocation OtherComp) (Math|Vector|GetForwardVector (Transformation|GetWorldRotation OtherComp)) true "CreateNewSectionForCap" "/Engine/MapTemplates/Materials/BasicAsset01.BasicAsset01"))
  (Variables|Default|SetSlicedMesh _outotherhalfprocmesh)
  (CallFunction|RepurposeNewMesh))

(event Custom|RepurposeNewMesh
  (Physics|SetSimulatePhysics (Variables|Default|GetSlicedMesh) true))

(event EventBeginPlay
  ;[1 1 1] Copy SM to ProcSM
  (Class|KismetProceduralMeshLibrary|CopyProceduralMeshfromStaticMeshComponent (Variables|Default|GetMesh2Slice) 0 (Variables|Default|GetProceduralMesh) true))

(fn ConstructionScript)